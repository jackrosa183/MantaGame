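; BP_Recovery is a recovery pickup that holds a passenger until a FlyingPawn collects it.
; On BeginPlay a timeline moves the actor vertically in a small offset above its spawn location.
; Overlapping its Cloud adds the passenger to the pawn's onboard list, switches its animation by passenger type and snaps it to the CargoZone.
; The actor then destroys itself; random placement within the cargo zone is still a noted to-do.
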(event OnComponentBeginOverlap(Cloud)
  (params (OverlappedComponent :type Primitive%20Component%20Object%20Reference) (OtherActor :type Actor%20Object%20Reference) (OtherComp :type Primitive%20Component%20Object%20Reference) (OtherBodyIndex :type Integer) (bFromSweep :type Boolean) (SweepResult :type Hit%20Result%20Structure%20%28by%20ref%29))
  (bind _attached_passenger (Variables|Default|Getattached%20passenger))
  (bind _attached_passenger_2 (Variables|Default|Getattached%20passenger))
  (bind _asflying_pawn (Utilities|Casting|CastToFlyingPawn OtherActor))
  ;[1 1 1] release passenger
  (Development|PrintString "save")
  (Utilities|Array|Add (Variables|/Game/FlyingBP/Blueprints/FlyingPawn.FlyingPawn_C|Geton%20board%20pepo _asflying_pawn) (Variables|Default|Getattached%20passenger))
  (Transformation|DetachFromActor _attached_passenger "KeepRelative" "KeepRelative" "KeepRelative")
  (Components|Animation|PlayAnimation (Variables|/Game/Blueprints/BP_Passenger.BP_Passenger_C|GetSkeletalMesh _attached_passenger_2) (Utilities|Select :Index (Variables|/Game/Blueprints/BP_Passenger.BP_Passenger_C|GetPassengerType _attached_passenger_2) :Option%200 "/Game/Animations/ANIM_Flower_Idle.ANIM_Flower_Idle" :Option%201 "/Game/Animation/ANIM_Flower_Idle.ANIM_Flower_Idle" :Option%202 "/Game/Animation/ANIM_Busi_Wobble.ANIM_Busi_Wobble" :Option%203 "/Game/Animation/ANIM_Busi_Wobble.ANIM_Busi_Wobble" :Option%204 "/Game/Animation/ANIM_Burg_Idle.ANIM_Burg_Idle" :Option%205 "/Game/Animation/ANIM_Burg_Idle.ANIM_Burg_Idle") false)
  ;[1 1 1] set random loc in cargo zone later
  (Transformation|AttachComponentToComponent _attached_passenger (Variables|/Game/FlyingBP/Blueprints/FlyingPawn.FlyingPawn_C|GetCargoZone _asflying_pawn) "None" "SnapToTarget" "KeepRelative" "KeepRelative" true)
  (Actor|DestroyActor))

(event EventBeginPlay
  (Variables|Default|Setspawn%20loc (Transformation|GetActorLocation))
  (bind _newtrack_0 (Timeline|Timeline_0 Play)
    (:Update
      (Transformation|SetActorLocation (Math|Vector|MakeVector (.x (Variables|Default|Getspawn%20loc)) (.y (Variables|Default|Getspawn%20loc)) (+ (.z (Variables|Default|Getspawn%20loc)) (Math|Float|Lerp 0.0 3e+01 _newtrack_0))) false false))))

(event EventTick
  (params (DeltaSeconds :type Float%20%28single-precision%29)))

(fn ConstructionScript)