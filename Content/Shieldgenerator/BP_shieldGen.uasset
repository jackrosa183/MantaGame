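; Shield generator Blueprint that deploys an expanding forcefield when its BuildField event is called.
; BuildField plays a charge sound at the skeletal mesh, then runs the Expand timeline to scale the forcefield uniformly up from zero.
; The same timeline raises the particle system to a target height, lerping from its current Z each update rather than a stored start.
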(event Custom|BuildField
  (bind _particlesystem (Variables|Default|GetParticleSystem))
  (Audio|PlaySoundatLocation "/Game/Sound/SFX_ShieldCharge.SFX_ShieldCharge" (Transformation|GetWorldLocation (Variables|Default|GetSkeletalMesh)) "0, 0, 0" 1.0 1.0 0.0 0 0 0)
  (bind _newtrack_0 (Timeline|Expand Play)
    (:Update
      (Transformation|SetWorldScale3D (Variables|Default|Getforcefield) (Math|Vector|MakeVector (Math|Float|Lerp 0.0 4e+01 _newtrack_0) (Math|Float|Lerp 0.0 4e+01 _newtrack_0) (Math|Float|Lerp 0.0 4e+01 _newtrack_0)))
      (Transformation|SetRelativeLocation _particlesystem (Math|Vector|MakeVector 0.0 0.0 (Math|Float|Lerp (.z (Variables|/Script/Engine.SceneComponent|GetRelativeLocation _particlesystem)) 485.0 _newtrack_0)) false false))))

(event EventBeginPlay)

(fn ConstructionScript)