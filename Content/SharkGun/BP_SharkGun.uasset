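; BP_SharkGun is a buildable turret that tracks the shark and fires BP_Harpoon projectiles at it.
; BeginPlay caches the first BP_Shark; the Construct event plays particles for three seconds, then shows the gun mesh and enables attacking.
; A fast looping timer rotates the root toward the shark's sphere.
; While attacking, Tick spawns and fires a harpoon every frame, as the random check's weight of 2.0 always passes.
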(event Custom|Construct
  (Components|Activation|Activate (Variables|Default|GetParticleSystem) false)
  (Components|Activation|Activate (Variables|Default|GetParticleSystem1) false)
  (Utilities|FlowControl|Delay 3.0)
  (Components|StaticMesh|SetStaticMesh (Variables|Default|GetStaticMesh) "/Game/SharkGun/SM_SharkGun.SM_SharkGun")
  (Components|Activation|Deactivate (Variables|Default|GetParticleSystem))
  (Components|Activation|Deactivate (Variables|Default|GetParticleSystem1))
  (CallFunction|Update)
  (Variables|Default|Setattack true))

(event Custom|Look%20at%20shark
  (Transformation|SetWorldRotation (Variables|Default|GetDefaultSceneRoot) (Math|Rotator|FindLookatRotation (Transformation|GetWorldLocation (Variables|Default|GetDefaultSceneRoot)) (Transformation|GetWorldLocation (Variables|/Game/Shark/BP_Shark.BP_Shark_C|GetSphere (Variables|Default|GetSharkTarget)))) false false))

(event Custom|Update
  (Utilities|Time|SetTimerbyEvent (delegate Custom|Look%20at%20shark) 0.01 true))

(event EventTick
  (params (DeltaSeconds :type Float%20%28single-precision%29))
  (if (Math|Random|RandomBoolwithWeight 2.0)
    (if (Variables|Default|Getattack)
      (bind _returnvalue (Game|SpawnActorfromClass "/Game/SharkGun/BP_Harpoon.BP_Harpoon_C" (Transformation|GetWorldTransform (Variables|Default|GetHarpoonSpawnLocation)) "Undefined" 0 0))
      (Default|Fire _returnvalue))))

(event EventBeginPlay
  (bind _returnvalue (Actor|GetActorOfClass "/Game/Shark/BP_Shark.BP_Shark_C"))
  (Variables|Default|SetSharkTarget _returnvalue))

(fn ConstructionScript
  (if (Variables|Default|Getisbuilt)
    (Components|StaticMesh|SetStaticMesh (Variables|Default|GetStaticMesh) "/Game/SharkGun/SM_SharkGun.SM_SharkGun")))