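; BP_Harpoon is a harpoon projectile that homes in on the shark, damages it and sticks to it.
; BeginPlay caches the BP_Sharkreal actor found in the level.
; Fire detaches the harpoon, targets the shark's root for homing, sets a forward unit velocity and activates ProjectileMovement.
; Overlapping a shark while AbleToDoDamage is set deals damage, clears the flag and attaches the harpoon to the cached shark.
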(event Custom|Fire
  (Development|PrintString "fire")
  (Transformation|DetachFromActor "KeepWorld" "KeepWorld" "KeepWorld")
  (Variables|/Script/Engine.ProjectileMovementComponent|SetHomingTargetComponent (Variables|Default|GetProjectileMovement) (Variables|/Game/Shark/BP_Sharkreal.BP_Sharkreal_C|GetDefaultSceneRoot (Variables|Default|Getshark)))
  (Variables|/Script/Engine.MovementComponent|SetVelocity (Variables|Default|GetProjectileMovement) (Math|Vector|Normalize (Math|Vector|GetForwardVector (Transformation|GetWorldRotation (Variables|Default|GetDefaultSceneRoot)))))
  (Components|Activation|Activate (Variables|Default|GetProjectileMovement) false))

(event EventBeginPlay
  (bind _returnvalue (Actor|GetActorOfClass "/Game/Shark/BP_Sharkreal.BP_Sharkreal_C"))
  (Variables|Default|Setshark _returnvalue))

(event Collision|EventActorBeginOverlap
  (params (OtherActor :type Actor%20Object%20Reference))
  (bind _asbp_sharkreal (Utilities|Casting|CastToBP_Sharkreal OtherActor))
  (if (Variables|Default|Getable%20to%20do%20damage?)
    ;[1 0 0.1081] add sound
    (Default|Damage _asbp_sharkreal 25.0)
    (Variables|Default|Setable%20to%20do%20damage? false)
    (Transformation|AttachActorToActor (Variables|Default|Getshark) "None" "KeepWorld" "KeepWorld" "KeepWorld" true)))

(fn ConstructionScript)