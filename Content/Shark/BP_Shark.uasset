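; BP_Shark is a flying shark actor that hunts sky stations needing an engineer.
; On BeginPlay it gathers unprotected BP_SkyStations and homes its projectile movement on the current one, advancing when its sphere overlaps a station.
; SpeedUp switches to a biting animation and raises the path timeline's rate.
; The spline-follow logic is disconnected, leaving Endtime, which gates hiding overlapped non-tornado actors, never set here.
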(event OnComponentBeginOverlap(Sphere)
  (params (OverlappedComponent :type Primitive%20Component%20Object%20Reference) (OtherActor :type Actor%20Object%20Reference) (OtherComp :type Primitive%20Component%20Object%20Reference) (OtherBodyIndex :type Integer) (bFromSweep :type Boolean) (SweepResult :type Hit%20Result%20Structure%20%28by%20ref%29))
  (Utilities|Casting|CastToBP_SkyStation OtherActor)
  (CallFunction|NextCity)
  (Development|PrintString "next"))

(event Custom|Follow%20path)

(event Custom|Speed%20Up
  (Components|Timeline|SetPlayRate (Variables|Default|GetfollowTL) 0.8)
  (Components|Animation|PlayAnimation (Variables|Default|GetSkeletalMesh) "/Game/Shark/ANIM_Shark_biting__1_.ANIM_Shark_biting__1_" true))

(event Custom|find%20unprotected%20Cities
  (bind _outactors (Actor|GetAllActorsOfClass "/Game/Blueprints/BP_SkyStation.BP_SkyStation_C"))
  (for _array_element _outactors
    (if (Variables|/Game/Blueprints/BP_SkyStation.BP_SkyStation_C|GetneedsEngineer? _array_element)
      (Utilities|Array|Add (Variables|Default|Getunprotectedcities) _array_element)))
  (CallFunction|Hunt))

(event Custom|next%20city
  (Utilities|FlowControl|DoOnce false :!label _label
    (:Completed
      (Math|Integer|IncrementInt (Variables|Default|GetUnprotectedIndex)
        (:%20%20
          (CallFunction|Hunt)
          (goto _label Reset))))))

(event Custom|hunt
  (bind _unprotectedindex (Variables|Default|GetUnprotectedIndex))
  (bind _unprotectedcities (Variables|Default|Getunprotectedcities))
  (bind _output (Utilities|Array|Get(acopy) _unprotectedcities _unprotectedindex))
  (Utilities|IsValid _output
    (:Is%20Valid
      (bind _output_get (Variables|Default|SetCurrentCityTarget _output))
      (Variables|/Script/Engine.ProjectileMovementComponent|SetHomingTargetComponent (Variables|Default|GetProjectileMovement) (Variables|/Game/Blueprints/BP_SkyStation.BP_SkyStation_C|GetDefaultSceneRoot _output_get)))))

(event EventBeginPlay
  (Components|Animation|PlayAnimation (Variables|Default|GetSkeletalMesh) "/Game/Shark/ANIM_Shark_flyingtest.ANIM_Shark_flyingtest" true)
  (CallFunction|FindUnprotectedCities))

(event Collision|EventActorBeginOverlap
  (params (OtherActor :type Actor%20Object%20Reference))
  (Utilities|FlowControl|Sequence
    (:then_0
      (if (Variables|Default|Getendtime?)
        (Utilities|Casting|CastToBP_TornadoClass (Utilities|GetClass OtherActor)
          (:CastFailed
            (Rendering|SetActorHiddenInGame OtherActor true)))))))

(fn ConstructionScript)