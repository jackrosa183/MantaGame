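; Flying shark actor that stages an end sequence, hunting down SkyStations that still need an engineer.
; It rides a spline via timeline, then switches to biting animation and roar music, gathers those stations and cuts to a tracking EndCamera.
; Homing projectile movement steers it to each target, hiding it on overlap before advancing, along with most other actors it touches.
; Damage only lowers health and prints a debug message.
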(event OnComponentBeginOverlap(Sphere)
  (params (OverlappedComponent :type Primitive%20Component%20Object%20Reference) (OtherActor :type Actor%20Object%20Reference) (OtherComp :type Primitive%20Component%20Object%20Reference) (OtherBodyIndex :type Integer) (bFromSweep :type Boolean) (SweepResult :type Hit%20Result%20Structure%20%28by%20ref%29))
  (bind _asbp_sky_station (Utilities|Casting|CastToBP_SkyStation OtherActor)
    (:then
      (if (== _asbp_sky_station (Variables|Default|GetCurrentCityTarget))
        (Rendering|SetActorHiddenInGame _asbp_sky_station true)
        (CallFunction|NextCity)
        (Development|PrintString "next")))
    (:CastFailed
      (Utilities|FlowControl|Sequence
        (:then_0
          (Utilities|Casting|CastToBP_Sharkreal OtherActor
            (:CastFailed
              (if (Variables|Default|Getendtime?)
                (Utilities|Casting|CastToBP_Tornado OtherActor
                  (:CastFailed
                    (Rendering|SetActorHiddenInGame OtherActor true)))))))))))

(event Custom|Follow%20path
  (bind _skeletalmesh (Variables|Default|GetSkeletalMesh))
  (bind _path (Variables|Default|GetPATH))
  (bind _spline (Variables|/Game/Blueprints/BP_Path.BP_Path_C|GetSpline _path))
  (Components|Timeline|SetPlayRate (Variables|Default|GetfollowTL) (Variables|Default|Getsplinerate))
  (bind _newtrack_0 (Timeline|followTL Play)
    (:Update
      (Transformation|SetActorTransform (Math|Transform|MakeTransform (Spline|GetLocationatDistanceAlongSpline _spline (Math|Float|Lerp 0.0 (Spline|GetSplineLength _spline) _newtrack_0) "World") (Spline|GetRotationatDistanceAlongSpline _spline (Math|Float|Lerp 0.0 (Spline|GetSplineLength _spline) _newtrack_0) "World") "1,1,1")))
    (:Finished
      (Components|Animation|PlayAnimation _skeletalmesh "/Game/Shark/ANIM_Shark_biting__1_.ANIM_Shark_biting__1_" true)
      (Components|Timeline|SetPlayRate _skeletalmesh 1e+01)
      (CallFunction|FindUnprotectedCities)
      (Variables|Default|Setendtime? true))))

(event Custom|damage
  (params (damage%20amount :type Float%20%28single-precision%29))
  (Variables|Default|Sethealth (- (Variables|Default|Gethealth) damage%20amount))
  ;[1 1 1] or animation
  (CallFunction|SomeDamageEffect))

(event Custom|find%20unprotected%20Cities
  (Utilities|HandleAudio (stale EventBeginPlay _returnvalue))
  (bind _outactors (Actor|GetAllActorsOfClass "/Game/Blueprints/BP_SkyStation.BP_SkyStation_C"))
  (for _array_element _outactors
    (if (Variables|/Game/Blueprints/BP_SkyStation.BP_SkyStation_C|GetneedsEngineer? _array_element)
      (Utilities|Array|Add (Variables|Default|Getunprotectedcities) _array_element)))
  (CallFunction|Hunt))

(event Custom|next%20city
  (Utilities|FlowControl|DoOnce false :!label _label
    (:Completed
      (Math|Integer|IncrementInt (Variables|Default|GetUnprotectedIndex)
        (:%20%20
          (CallFunction|Hunt)
          (goto _label Reset))))))

(event Custom|hunt
  (bind _unprotectedindex (Variables|Default|GetUnprotectedIndex))
  (bind _unprotectedcities (Variables|Default|Getunprotectedcities))
  (bind _output (Utilities|Array|Get(acopy) _unprotectedcities _unprotectedindex))
  (Game|Player|SetViewTargetwithBlend (Game|GetPlayerController 0) (Variables|Default|GetEndCamera) 0.5 "VTBlend_Linear" 0.0 false)
  (Utilities|IsValid _output
    (:Is%20Valid
      (bind _output_get (Variables|Default|SetCurrentCityTarget _output))
      (Variables|/Script/Engine.ProjectileMovementComponent|SetHomingTargetComponent (Variables|Default|GetProjectileMovement) (Variables|/Game/Blueprints/BP_SkyStation.BP_SkyStation_C|GetDefaultSceneRoot _output_get)))))

(event Custom|some%20damage%20effect
  (Development|PrintString "shark: ouch" true true "(R=1.000000,G=0.000000,B=0.094240,A=1.000000)" 5.0))

(event EventBeginPlay
  (Components|Animation|PlayAnimation (Variables|Default|GetSkeletalMesh) "/Game/Shark/ANIM_Shark_flyingtest.ANIM_Shark_flyingtest" true)
  (CallFunction|FollowPath)
  (bind _returnvalue (Audio|CreateSound2D "/Game/Sound/Music/Music_Jazz_2.Music_Jazz_2" 1.0 1.0 0.0 0))
  (Audio|Components|Audio|FadeIn _returnvalue 1.0 1.0 0.0 "Linear" :!class /Script/Engine.AudioComponent))

(event EventTick
  (params (DeltaSeconds :type Float%20%28single-precision%29))
  (Transformation|SetActorRotation (Variables|Default|GetEndCamera) (Math|Rotator|FindLookatRotation (Transformation|GetWorldLocation (Variables|/Script/Engine.Actor|GetRootComponent (Variables|Default|GetEndCamera))) (Transformation|GetWorldLocation (Variables|Default|GetDefaultSceneRoot)))))

(fn ConstructionScript)