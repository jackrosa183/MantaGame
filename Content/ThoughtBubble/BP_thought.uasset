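; BP_thought is a thought bubble actor that periodically shows a particle effect with a sound.
; ActivateThought switches the particles off, waits briefly, activates them and plays the audio, then deactivates them after another short delay.
; BeginPlay runs this once, and Tick repeats it through a longer Delay, which acts as a repeating timer because calls during the countdown are ignored.
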(event Custom|ActivateThought
  (Components|Activation|Deactivate (Variables|Default|GetParticleSystem))
  (Utilities|FlowControl|Delay 3.0)
  (Components|Activation|Activate (Variables|Default|GetParticleSystem) false)
  (Audio|Components|Audio|Play (Variables|Default|GetAudio) 0.0)
  (Utilities|FlowControl|Delay 3.0)
  (Components|Activation|Deactivate (Variables|Default|GetParticleSystem)))

(event EventBeginPlay
  (CallFunction|ActivateThought))

(event Collision|EventActorBeginOverlap
  (params (OtherActor :type Actor%20Object%20Reference)))

(event EventTick
  (params (DeltaSeconds :type Float%20%28single-precision%29))
  (Utilities|FlowControl|Delay 15.0)
  (CallFunction|ActivateThought))

(fn ConstructionScript)