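; BP_Guide is a cone guide marker that bobs vertically and resizes with the player's distance.
; On BeginPlay it caches the cone's original scale and a FlyingPawn reference, then starts the Bob timeline, which adds a Z offset to the current position each update.
; Tick scales the cone by clamped, normalized distance, so it shrinks as the pawn approaches and reaches full size when far away.
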(event EventBeginPlay
  (bind _cone (Variables|Default|GetCone))
  (bind _returnvalue (Transformation|GetWorldLocation _cone))
  (Variables|Default|SetogScale (Transformation|GetWorldScale (Variables|Default|GetCone)))
  (bind _outactors (Actor|GetAllActorsOfClass "/Game/FlyingBP/Blueprints/FlyingPawn.FlyingPawn_C"))
  (for _array_element _outactors
    (Variables|Default|SetPlayer _array_element))
  (bind _bobtrack (Timeline|Bob Play)
    (:Update
      (Transformation|SetWorldLocation _cone (Math|Vector|MakeVector (.x _returnvalue) (.y _returnvalue) (+ (.z _returnvalue) (* _bobtrack 3.0))) false false))))

(event EventTick
  (params (DeltaSeconds :type Float%20%28single-precision%29))
  (bind _self self)
  (bind _player (Variables|Default|GetPlayer))
  (bind _returnvalue (Transformation|GetDistanceTo _player _self))
  (bind _returnvalue_2 (Math|Float|Clamp(Float) _returnvalue 0.0 1e+04))
  (bind _returnvalue_3 (/ _returnvalue_2 1e+04))
  (Transformation|SetWorldScale3D (Variables|Default|GetCone) (* (Math|Vector|MakeVector _returnvalue_3 _returnvalue_3 _returnvalue_3) (Variables|Default|GetogScale))))

(fn ConstructionScript)