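; Eyeball actor that attaches itself to the first BP_Tornado in the level, bobs vertically and stares at the player's FlyingPawn.
; On BeginPlay, a looping MoveComponentTo and FlipFlop eases the Eyeball component between upward and downward offsets from its current position.
; FacePlayer smoothly interpolates the actor's pitch and yaw toward the pawn, re-calling itself after a tiny Delay instead of using Tick.
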(event Custom|FacePlayer
  (bind _returnvalue (Transformation|GetActorLocation))
  (bind _returnvalue_2 (Utilities|Time|GetWorldDeltaSeconds))
  (bind _returnvalue_3 (Transformation|GetActorRotation))
  (bind _char_ref (Variables|Default|GetChar%20Ref))
  (bind _returnvalue_4 (Transformation|GetActorLocation _char_ref))
  (bind _returnvalue_5 (Math|Rotator|FindLookatRotation _returnvalue _returnvalue_4))
  (bind _returnvalue_6 (Math|Interpolation|RInterpTo _returnvalue_3 _returnvalue_5 _returnvalue_2 1e+01))
  (Transformation|SetActorRotation (Math|Rotator|MakeRotator 0.0 (.pitch _returnvalue_6) (.yaw _returnvalue_6)))
  (Utilities|FlowControl|Delay 0.001)
  (CallFunction|FacePlayer))

(event EventBeginPlay
  (bind _eyeball (Variables|Default|GetEyeball))
  (bind _relativelocation (Variables|/Script/Engine.SceneComponent|GetRelativeLocation _eyeball))
  (Utilities|FlowControl|Sequence
    (:then_0
      (Components|MoveComponentTo _eyeball (Math|Vector|SelectVector (+ _relativelocation "0, 0,500.000000") (- _relativelocation "0, 0,500.000000") (Variables|Default|GetRepeat)) "0, 0, 0" true true 3.0 false :!label _label)
      (Utilities|FlowControl|FlipFlop
        (:A
          (Variables|Default|Setrepeat true)
          (goto _label))
        (:B
          (Variables|Default|Setrepeat false)
          (goto _label))))
    (:then_1
      (bind _asflying_pawn (Utilities|Casting|CastToFlyingPawn (Game|Player|GetPlayerPawn 0)))
      (Variables|Default|SetChar%20Ref _asflying_pawn)
      (CallFunction|FacePlayer)
      (bind _outactors (Actor|GetAllActorsOfClass "/Game/Blueprints/BP_Tornado.BP_Tornado_C"))
      (Transformation|AttachActorToActor (Utilities|Array|Get(acopy) _outactors) "None" "KeepRelative" "KeepRelative" "KeepRelative" true))))

(event Collision|EventActorBeginOverlap
  (params (OtherActor :type Actor%20Object%20Reference)))

(event EventTick
  (params (DeltaSeconds :type Float%20%28single-precision%29)))

(fn ConstructionScript)