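; BP_StarTrinket is a pickup that adds game time when it overlaps the FlyingPawn's cargo box, with confetti and a UI notification.
; Timelines fade the trinket and ramp the pawn's glow and speed up, then down after a delay, compounding speed from its current value each update.
; It hides and sets Pickedup only after the notification delay.
; The construction script applies the configurable skeletal mesh and animation.
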(event OnComponentBeginOverlap(Box)
  (params (OverlappedComponent :type Primitive%20Component%20Object%20Reference) (OtherActor :type Actor%20Object%20Reference) (OtherComp :type Primitive%20Component%20Object%20Reference) (OtherBodyIndex :type Integer) (bFromSweep :type Boolean) (SweepResult :type Hit%20Result%20Structure%20%28by%20ref%29))
  (if (not (Variables|Default|GetPickedup?))
    (bind _asflying_pawn (Utilities|Casting|CastToFlyingPawn OtherActor))
    (Variables|Default|Setflyingpawn _asflying_pawn)
    (if (== OtherComp (Variables|/Game/FlyingBP/Blueprints/FlyingPawn.FlyingPawn_C|Getcargobox _asflying_pawn))
      (bind _asflying_game_mode (Utilities|Casting|CastToFlyingGameMode (Game|GetGameMode)))
      (Variables|/Game/FlyingBP/Blueprints/FlyingGameMode.FlyingGameMode_C|SetGameTime _asflying_game_mode (+ (Variables|/Game/FlyingBP/Blueprints/FlyingGameMode.FlyingGameMode_C|GetGameTime _asflying_game_mode) 15.0))
      (Components|Activation|Activate (Variables|Default|GetConfetti) false)
      (CallFunction|MakeNotification)
      (bind _returnvalue (Rendering|Material|CreateDynamicMaterialInstance (Variables|Default|GetSkeletalMesh) 0 "/Game/Materials/M-FadeItem1.M-FadeItem1" "None" :!class /Script/Engine.PrimitiveComponent))
      (bind _returnvalue_2 (Rendering|Material|CreateDynamicMaterialInstance (Variables|/Game/FlyingBP/Blueprints/FlyingPawn.FlyingPawn_C|GetSkeletalMesh (Variables|Default|Getflyingpawn)) 0 "/Game/NewManta/M_Manta.M_Manta" "None" :!class /Script/Engine.PrimitiveComponent))
      (bind _newtrack_0 (Timeline|Transition Play)
        (:Update
          (Rendering|Material|SetScalarParameterValue _returnvalue "Fade" _newtrack_0 :!class /Script/Engine.MaterialInstanceDynamic)
          (Rendering|Material|SetScalarParameterValue _returnvalue_2 "GlowMulti" (Math|Float|Lerp 0.0 1e+02 _newtrack_0) :!class /Script/Engine.MaterialInstanceDynamic)
          (Variables|/Game/FlyingBP/Blueprints/FlyingPawn.FlyingPawn_C|SetCurrent%20forward%20speed (Variables|Default|Getflyingpawn) (Math|Float|Lerp (Variables|/Game/FlyingBP/Blueprints/FlyingPawn.FlyingPawn_C|GetCurrent%20forward%20speed (Variables|Default|Getflyingpawn)) (+ (Variables|/Game/FlyingBP/Blueprints/FlyingPawn.FlyingPawn_C|GetCurrent%20forward%20speed (Variables|Default|Getflyingpawn)) 5e+01) _newtrack_0)))
        (:Finished
          (Utilities|FlowControl|Delay 5.0)
          (bind _newtrack_0_2 (Timeline|Timeline_0 Play)
            (:Update
              (Rendering|Material|SetScalarParameterValue _returnvalue_2 "GlowMulti" (Math|Float|Lerp 1e+02 0.0 _newtrack_0_2) :!class /Script/Engine.MaterialInstanceDynamic)
              (Variables|/Game/FlyingBP/Blueprints/FlyingPawn.FlyingPawn_C|SetCurrent%20forward%20speed (Variables|Default|Getflyingpawn) (Math|Float|Lerp (Variables|/Game/FlyingBP/Blueprints/FlyingPawn.FlyingPawn_C|GetCurrent%20forward%20speed (Variables|Default|Getflyingpawn)) (- (Variables|/Game/FlyingBP/Blueprints/FlyingPawn.FlyingPawn_C|GetCurrent%20forward%20speed (Variables|Default|Getflyingpawn)) 1e+02) _newtrack_0_2)))))))))

(event Custom|MakeNotification
  (bind _returnvalue (UserInterface|CreateWidget "/Game/UI/UI_Trinket_Notification.UI_Trinket_Notification_C"))
  (UserInterface|Viewport|AddtoViewport _returnvalue 0)
  (Utilities|FlowControl|Delay 3.0)
  (Rendering|SetActorHiddenInGame true)
  (Variables|Default|SetPickedup? true))

(event EventBeginPlay)

(fn ConstructionScript
  (Class|SkinnedMeshComponent|SetSkeletalMesh (Variables|Default|GetSkeletalMesh) (Variables|Default|Getskeletal) true)
  (Components|Animation|OverrideAnimationData (Variables|Default|GetSkeletalMesh) (Variables|Default|Getanimation) true true 0.0 1.0))