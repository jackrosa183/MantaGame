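; BP_Passenger is a station passenger whose PassengerType picks its skeletal mesh, animations and thought-bubble material.
; It binds to its BirthStation's move-up event, stepping forward in timed increments while not boarded.
; After a short randomized fall, it stops physics, spawns and attaches to a BP_Recovery actor, and plays a balloon animation.
; A Delay on Tick paces random thought-bubble emitters with sound; other events play boarding, fall and celebration sounds.
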(event Custom|queue%20move%20up
  ;[1 1 1] attached thus skystation orientation
  (if (not (Variables|Default|Getboarded?))
    (if (< (Variables|Default|GetCounter) 20) :!label _label
      (Transformation|AddActorLocalOffset (Math|Vector|MakeVector 0.0 1.0 0.0) false false)
      (Math|Integer|IncrementInt (Variables|Default|GetCounter)
        (:%20%20
          (Utilities|FlowControl|Delay 0.025)
          (goto _label)))
      (else
        (Variables|Default|SetCounter 0)))))

(event Custom|I've%20fallen%20and%20I%20can't%20get%20up
  ;[1 1 1] fall for a bit
  (Utilities|FlowControl|Delay (Math|Random|RandomFloatinRange 1.0 2.0))
  ;[1 1 1] set char mesh as root for this
  (Physics|SetSimulatePhysics (Variables|Default|GetSkeletalMesh) false)
  (bind _returnvalue (Game|SpawnActorfromClass "/Game/passenger_recovery/BP_Recovery.BP_Recovery_C" (Math|Transform|MakeTransform (Transformation|GetActorLocation) "0, 0, 0" "1,1,1") "AlwaysSpawn" 0 self 0))
  (Transformation|AttachActorToActor _returnvalue "None" "SnapToTarget" "KeepWorld" "KeepWorld" true)
  (Components|Animation|PlayAnimation (Variables|Default|GetSkeletalMesh) (Utilities|Select :Index (Variables|Default|GetPassengerType) :Option%200 "/Game/ANIM_Flower_Balloon.ANIM_Flower_Balloon" :Option%201 "/Game/ANIM_Flower_Balloon.ANIM_Flower_Balloon" :Option%202 "/Game/ANIM_Business_Balloon.ANIM_Business_Balloon" :Option%203 "/Game/ANIM_Business_Balloon.ANIM_Business_Balloon" :Option%204 "/Game/ANIM_Burger_Balloon.ANIM_Burger_Balloon" :Option%205 "/Game/ANIM_Burger_Balloon.ANIM_Burger_Balloon") true)
  ;[1 1 1] set here or on retrieveal
  (Transformation|SetActorRotation "0, 0, 0"))

(event Custom|PlayIdles
  (bind _skeletalmesh (Variables|Default|GetSkeletalMesh))
  (Components|Animation|PlayAnimation _skeletalmesh (Utilities|Select :Index (Variables|Default|GetPassengerType) :Option%200 "/Game/Animations/ANIM_Flower_Idle.ANIM_Flower_Idle" :Option%201 "/Game/Animation/ANIM_Flower_Idle.ANIM_Flower_Idle" :Option%202 "/Game/Animation/ANIM_Busi_Wobble.ANIM_Busi_Wobble" :Option%203 "/Game/Animation/ANIM_Busi_Wobble.ANIM_Busi_Wobble" :Option%204 "/Game/Animation/ANIM_Burg_Idle.ANIM_Burg_Idle" :Option%205 "/Game/Animation/ANIM_Burg_Idle.ANIM_Burg_Idle") true)
  (Transformation|SetRelativeScale3D _skeletalmesh "0.300000,0.300000,0.300000"))

(event Custom|PlayBoardingSound
  (Audio|PlaySoundatLocation (Variables|Default|GetBoardingSoundCue) (Transformation|GetWorldLocation (Variables|Default|GetSkeletalMesh)) "0, 0, 0" 1.0 1.0 0.0 0 0 0))

(event Custom|PlayFallSound
  (Audio|PlaySoundatLocation (Variables|Default|GetFallSoundCue) (Transformation|GetWorldLocation (Variables|Default|GetSkeletalMesh)) "0, 0, 0" 1.0 1.0 0.0 0 0 0))

(event Custom|Play%20Celebration%20Sound
  (Audio|PlaySoundatLocation "/Game/Sound/CelebrationCue.CelebrationCue" (Transformation|GetWorldLocation (Variables|Default|GetSkeletalMesh)) "0, 0, 0" 1.0 1.0 0.0 0 0 0))

(event Custom|particle%20test)

(event EventBeginPlay
  (EventDispatchers|BindEventtoMoveUpYall (Variables|Default|Getbirth%20station) (delegate Custom|queue%20move%20up))
  (CallFunction|PlayIdles)
  (CallFunction|ParticleTest))

(event Collision|EventActorBeginOverlap
  (params (OtherActor :type Actor%20Object%20Reference)))

(event EventTick
  (params (DeltaSeconds :type Float%20%28single-precision%29))
  (Utilities|FlowControl|Delay (Math|Random|RandomFloatinRange 1e+01 15.0))
  (if (Math|Random|RandomBoolwithWeight 0.5)
    (Audio|PlaySoundatLocation "/Game/Sound/BoardingCue.BoardingCue" (Transformation|GetWorldLocation (Variables|Default|GetSkeletalMesh)) "0, 0, 0" 1.0 1.0 0.0 0 0 0)
    (bind _returnvalue (Effects|SpawnEmitterAttached "/Game/ThoughtBubble/P_Thought.P_Thought" (Variables|Default|GetScene) "None" "0, 0,50.000000" "0, 0, 0" "1.000000,1.000000,1.000000" "SnapToTarget"))
    (Rendering|Material|SetMaterial _returnvalue 0 (Utilities|Select :Index (Variables|Default|GetPassengerType) :Option%200 "/Game/ThoughtBubble/M_ThoughtBubble.M_ThoughtBubble" :Option%201 "/Game/ThoughtBubble/M_Thought_FlowerB.M_Thought_FlowerB" :Option%202 "/Game/ThoughtBubble/M_Thought_BusA.M_Thought_BusA" :Option%203 "/Game/ThoughtBubble/M_Thought_BusB.M_Thought_BusB" :Option%204 "/Game/ThoughtBubble/M_ThoughtFoodA.M_ThoughtFoodA" :Option%205 "/Game/ThoughtBubble/M_ThoughtFoodB.M_ThoughtFoodB"))))

(fn ConstructionScript
  (Class|SkinnedMeshComponent|SetSkeletalMesh (Variables|Default|GetSkeletalMesh) (Utilities|Select :Index (Variables|Default|GetPassengerType) :Option%200 "/Game/passenger_fbx/BotanicalBoyRIGGED.BotanicalBoyRIGGED" :Option%201 "/Game/passenger_fbx/BotanicalBoyRIGGED.BotanicalBoyRIGGED" :Option%202 "/Game/Animation/SK_Businessman.SK_Businessman" :Option%203 "/Game/Animation/SK_Businessman.SK_Businessman" :Option%204 "/Game/passenger_fbx/BurgerBoyRIGGED.BurgerBoyRIGGED" :Option%205 "/Game/passenger_fbx/BurgerBoyRIGGED.BurgerBoyRIGGED") true)
  (Transformation|AddActorLocalRotation (Math|Rotator|MakeRotator 0.0 0.0 9e+01) false false))