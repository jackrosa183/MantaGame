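; Tornado actor that travels along the spline of a referenced Path while its mesh spins.
; On BeginPlay the MoveTornado timeline plays at a rate set by MoveSpeed, mapping its Alpha to a distance along the spline to place the actor in world space.
; Each Tick increments a yaw counter on TornadoMesh, so spin speed depends on frame rate.
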(event EventBeginPlay
  (Components|Timeline|SetPlayRate (Variables|Default|GetMoveTornado) (Variables|Default|GetMoveSpeed))
  (bind _alpha (Timeline|MoveTornado Play)
    (:Update
      (Transformation|SetActorTransform (Math|Transform|MakeTransform (Spline|GetLocationatDistanceAlongSpline (Variables|/Game/Blueprints/BP_StormPath.BP_StormPath_C|GetSpline (Variables|Default|GetPath)) (Math|Float|Lerp 0.0 (Spline|GetSplineLength (Variables|/Game/Blueprints/BP_StormPath.BP_StormPath_C|GetSpline (Variables|Default|GetPath))) _alpha) "World") "0, 0, 0" "1,1,1")))))

(event EventTick
  (params (DeltaSeconds :type Float%20%28single-precision%29))
  (bind _result (Math|Float|IncrementFloat (Variables|Default|GetRotationfloat))
    (:%20%20
      (Transformation|SetRelativeRotation (Variables|Default|GetTornado_Mesh) (Math|Rotator|MakeRotator 0.0 0.0 _result) false false))))

(fn ConstructionScript)