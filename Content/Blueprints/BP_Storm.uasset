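; Storm actor that rains on the flying pawn and can knock its passengers off with lightning.
; While the pawn's IsInSafeCloud flag and StormActivated are set, Tick interpolates the storm toward the pawn's StormAttach point.
; A one-second Delay paces a coin-flip strike that briefly beams lightning at a random passenger and calls FalloffWithTarget.
; Beam target and falling passenger come from separate Random calls, so they can differ.
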(event EventTick
  (params (DeltaSeconds :type Float%20%28single-precision%29))
  (bind _flyingpawn (Variables|Default|GetFlyingPawn))
  (bind _on_board_pepo (Variables|/Game/FlyingBP/Blueprints/FlyingPawn.FlyingPawn_C|Geton%20board%20pepo _flyingpawn))
  (bind _outitem (Utilities|Array|Random _on_board_pepo))
  (if (Variables|/Game/FlyingBP/Blueprints/FlyingPawn.FlyingPawn_C|GetisInSafeCloud? (Variables|Default|GetFlyingPawn))
    (if (Variables|Default|GetStormActivated)
      (Utilities|FlowControl|Sequence
        (:then_0
          (Transformation|SetActorLocation (Math|Interpolation|VInterpTo (Transformation|GetActorLocation) (Transformation|GetWorldLocation (Variables|/Game/FlyingBP/Blueprints/FlyingPawn.FlyingPawn_C|GetStormAttach (Variables|Default|GetFlyingPawn))) DeltaSeconds 0.0) false false)
          (Components|Activation|Activate (Variables|Default|GetRain) false))
        (:then_1
          (Utilities|FlowControl|Delay 1.0)
          (if (> (Utilities|Array|Length (Variables|/Game/FlyingBP/Blueprints/FlyingPawn.FlyingPawn_C|Geton%20board%20pepo (Variables|Default|GetFlyingPawn))) 0)
            (if (Math|Random|RandomBoolwithWeight 0.5)
              (Components|Activation|Activate (Variables|Default|GetLightningParticle) false)
              (Class|ParticleSystemComponent|SetBeamTargetPoint (Variables|Default|GetLightningParticle) 0 (Transformation|GetWorldLocation (Variables|/Game/Blueprints/BP_Passenger.BP_Passenger_C|GetSkeletalMesh _outitem)))
              (Default|FalloffwithTarget (Variables|Default|GetFlyingPawn) _outitem)
              (Utilities|FlowControl|Delay 0.5)
              (Components|Activation|Deactivate (Variables|Default|GetLightningParticle))))))
      (else
        (Components|Activation|Deactivate (Variables|Default|GetRain))))))

(event EventBeginPlay
  (Components|Activation|Deactivate (Variables|Default|GetLightningParticle))
  (Components|Activation|Deactivate (Variables|Default|GetRain)))

(fn ConstructionScript)