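; BP_Whale is an actor that plays a looping whale animation and moves continuously along a circular path.
; On BeginPlay the skeletal mesh starts the looping animation.
; Each Tick adds a local forward offset from ForwardSpeed and a local yaw from TurnSpeed, both scaled by delta time, without sweep, so movement ignores collision.
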(event EventBeginPlay
  (Components|Animation|PlayAnimation (Variables|Default|GetSkeletalMesh) "/Game/Whale/SK_Character_Whale_Anim.SK_Character_Whale_Anim" true))

(event Collision|EventActorBeginOverlap
  (params (OtherActor :type Actor%20Object%20Reference)))

(event EventTick
  (params (DeltaSeconds :type Float%20%28single-precision%29))
  (Transformation|AddActorLocalOffset (Math|Vector|MakeVector (* DeltaSeconds (Variables|Default|GetForwardSpeed)) 0.0 0.0) false false)
  (Transformation|AddActorLocalRotation (Math|Rotator|MakeRotator 0.0 0.0 (* DeltaSeconds (Variables|Default|GetTurnSpeed))) false false))

(fn ConstructionScript)