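; Sky station where the FlyingPawn lands to drop off and pick up passengers.
; It spawns a queue of random passenger types, excluding its own BuildingTypes.
; Landing-zone overlap locks input, switches camera and timeline-lerps the pawn in, then releases matching passengers into physics and boards queued ones individually until capacity, before restoring control.
; Exiting the zone clears the queue array, spawns new passengers and re-arms landing after a delay.
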(event OnComponentEndOverlap(LandingZone)
  (params (OverlappedComponent :type Primitive%20Component%20Object%20Reference) (OtherActor :type Actor%20Object%20Reference) (OtherComp :type Primitive%20Component%20Object%20Reference) (OtherBodyIndex :type Integer))
  (bind _returnvalue (Game|GetPlayerController 0))
  (Utilities|Casting|CastToFlyingPawn OtherActor)
  (Utilities|FlowControl|DoOnce false :!label _label
    (:Completed
      (Utilities|Array|Clear (Variables|Default|Getstationpepo))
      ;[1 0 0.02432] Destroy too
      (CallFunction|SpawnPassengers)
      (Utilities|FlowControl|Delay 3.0)
      (Variables|Default|SetCanLandAgain? true)
      (Utilities|FlowControl|Sequence
        (:then_0
          (Utilities|FlowControl|DoOnce false) ; enters at Reset
        )
        (:then_1
          (goto _label Reset))))))

(event OnComponentBeginOverlap(LandingZone)
  (params (OverlappedComponent :type Primitive%20Component%20Object%20Reference) (OtherActor :type Actor%20Object%20Reference) (OtherComp :type Primitive%20Component%20Object%20Reference) (OtherBodyIndex :type Integer) (bFromSweep :type Boolean) (SweepResult :type Hit%20Result%20Structure%20%28by%20ref%29))
  (bind _returnvalue (Game|GetPlayerController 0))
  (Utilities|FlowControl|DoOnce false
    (:Completed
      (if (Variables|Default|GetCanLandAgain?)
        (Utilities|Casting|CastToFlyingPawn OtherActor)
        (Variables|Default|SetCanLandAgain? false)
        (Input|DisableInput (Variables|Default|GetFlyingPawn) _returnvalue)
        (Game|Player|SetViewTargetwithBlend _returnvalue (Variables|Default|GetLandingCam) (Variables|Default|GetLandingCamBlendTime) "VTBlend_Linear" 0.0 false)
        (Variables|/Game/FlyingBP/Blueprints/FlyingPawn.FlyingPawn_C|SetIsFlying (Variables|Default|GetFlyingPawn) false)
        (CallFunction|LandAnim)))))

(event Custom|LandAnim
  (bind _flyingpawn (Variables|Default|GetFlyingPawn))
  (bind _landcamlocation (Variables|Default|GetLandCamLocation))
  (bind _newtrack_0 (Timeline|Move%20character PlayFromStart)
    (:Update
      (Transformation|SetActorLocation _flyingpawn (Math|Vector|Lerp(Vector) (Transformation|GetActorLocation _flyingpawn) (Transformation|GetWorldLocation _landcamlocation) _newtrack_0) false false)
      (Transformation|SetActorRotation _flyingpawn (Math|Rotator|Lerp(Rotator) (Transformation|GetActorRotation _flyingpawn) (Transformation|GetWorldRotation _landcamlocation) _newtrack_0)))
    (:Finished
      (Development|PrintString "boarding")
      (if (> (CallFunction|OnboardPeopleSize) 0)
        (CallFunction|Unloading)
        (Utilities|FlowControl|Delay 5.0)
        (CallFunction|Boarding)
        (else
          (CallFunction|Boarding))))))

(event Custom|ResetLanding)

(event Custom|boarding
  (bind _flyingpawn (Variables|Default|GetFlyingPawn))
  (bind _flyingpawn_2 (Variables|Default|GetFlyingPawn))
  (bind _stationpepo (Variables|Default|Getstationpepo))
  (bind _on_board_pepo (Variables|/Game/FlyingBP/Blueprints/FlyingPawn.FlyingPawn_C|Geton%20board%20pepo _flyingpawn))
  (if (< (CallFunction|OnboardPeopleSize) (Variables|/Game/FlyingBP/Blueprints/FlyingPawn.FlyingPawn_C|GetrayCapacity (Variables|Default|GetFlyingPawn))) :!label _label
    (bind _returnvalue (Utilities|Array|Add _on_board_pepo (Utilities|Array|Get(acopy) _stationpepo)))
    (Utilities|Array|RemoveIndex _stationpepo)
    ;[1 1 1] board animation here
    (Default|CallMoveUpYall)
    (Variables|Default|SetRand%20Loc (Default|GetRandLoc _flyingpawn_2))
    (bind _output_get (Variables|Default|SetLOC%20STORE (Transformation|GetWorldLocation (Variables|/Game/Blueprints/BP_Passenger.BP_Passenger_C|GetDefaultSceneRoot (Utilities|Array|Get(acopy) _on_board_pepo _returnvalue)))))
    (bind _alpha (Timeline|Alpha PlayFromStart)
      (:Update
        (Transformation|SetWorldLocation (Variables|/Game/Blueprints/BP_Passenger.BP_Passenger_C|GetDefaultSceneRoot (Utilities|Array|Get(acopy) _on_board_pepo _returnvalue)) (Math|Vector|Lerp(Vector) _output_get (+ (Transformation|GetWorldLocation (Variables|/Game/FlyingBP/Blueprints/FlyingPawn.FlyingPawn_C|GetCargoZone _flyingpawn_2)) (Variables|Default|GetRand%20Loc)) _alpha) false false))
      (:Finished
        (Transformation|DetachFromActor (Utilities|Array|Get(acopy) _on_board_pepo _returnvalue) "KeepWorld" "KeepRelative" "KeepRelative")
        (Transformation|AttachComponentToComponent (Utilities|Array|Get(acopy) _on_board_pepo _returnvalue) (Variables|/Game/FlyingBP/Blueprints/FlyingPawn.FlyingPawn_C|GetCargoZone (Variables|Default|GetFlyingPawn)) "None" "KeepWorld" "KeepRelative" "KeepRelative" true)
        (Variables|/Game/Blueprints/BP_Passenger.BP_Passenger_C|Setboarded? (Utilities|Array|Get(acopy) _on_board_pepo _returnvalue) true)
        (Utilities|FlowControl|Delay 0.5)
        (goto _label)))
    (else
      (Development|PrintString "boarding end")
      (|leavingstation))))

(event Custom|unloading
  (for _array_element (Variables|/Game/FlyingBP/Blueprints/FlyingPawn.FlyingPawn_C|Geton%20board%20pepo (Variables|Default|GetFlyingPawn))
    (if (Utilities|Array|ContainsItem (Variables|Default|GetBuildingTypes) (Variables|/Game/Blueprints/BP_Passenger.BP_Passenger_C|GetPassengerType _array_element))
      (Development|PrintString "Unloading")
      (Physics|SetSimulatePhysics (Variables|/Game/Blueprints/BP_Passenger.BP_Passenger_C|GetCharacter_mesh _array_element) true)
      ;[1 0 0] More Complex Removal
      (Utilities|Array|Add (Variables|Default|GetPeopleToRemove) _array_element)
      (Transformation|DetachFromActor _array_element "KeepRelative" "KeepRelative" "KeepRelative")))
  (for _array_element_2 (Variables|Default|GetPeopleToRemove)
    (Utilities|Array|RemoveItem (Variables|/Game/FlyingBP/Blueprints/FlyingPawn.FlyingPawn_C|Geton%20board%20pepo (Variables|Default|GetFlyingPawn)) _array_element_2))
  (Utilities|Array|Clear (Variables|Default|GetPeopleToRemove)))

(event EventBeginPlay
  (bind _returnvalue (Actor|GetActorOfClass "/Game/FlyingBP/Blueprints/FlyingPawn.FlyingPawn_C"))
  (Variables|Default|SetFlyingPawn _returnvalue)
  (for _array_element (Variables|Default|GetBuildingTypes)
    (Utilities|Array|RemoveItem (Variables|Default|GetSpawnablePepo) _array_element))
  ;[1 1 1] initialize queue
  (CallFunction|SpawnPassengers))

(fn ConstructionScript)

(fn SpawnPassengers
  (bind _queue_start_spot (Variables|Default|Getqueue%20start%20spot))
  (for _index (range 0 (- (Variables|Default|Getstation%20capacity) 1))
    (bind _returnvalue (Game|SpawnActorfromClass "/Game/Blueprints/BP_Passenger.BP_Passenger_C" (Math|Transform|MakeTransform (Math|Vector|MakeVector (+ (* _index 2e+01) (.x _queue_start_spot)) (.y _queue_start_spot) (.z _queue_start_spot)) "0, 0, 0" "1,1,1") "Undefined" 0 (.OutItem (Utilities|Array|Random (Variables|Default|GetSpawnablePepo))) self 0))
    (Utilities|Array|Add (Variables|Default|Getstationpepo) _returnvalue)
    (Transformation|AttachActorToActor _returnvalue self "None" "KeepRelative" "KeepRelative" "KeepRelative" true))
  (return))

(fn OnboardPeopleSize
  (return (Utilities|Array|Length (Variables|/Game/FlyingBP/Blueprints/FlyingPawn.FlyingPawn_C|Geton%20board%20pepo (Variables|Default|GetFlyingPawn)))))