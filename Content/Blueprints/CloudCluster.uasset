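; Cloud cluster actor that randomizes its cloud meshes at BeginPlay and can show lightning or a safe-cloud material.
; Construction script applies the safe material to "Cloud"-tagged meshes when IsSafeCloud is set.
; With StormWLightning on, Tick uses random delays to briefly flash a downward beam.
; Collider overlaps with a FlyingPawn's Cargobox toggle IsInSafeCloud, without checking IsSafeCloud.
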(event OnComponentBeginOverlap(Collider)
  (params (OverlappedComponent :type Primitive%20Component%20Object%20Reference) (OtherActor :type Actor%20Object%20Reference) (OtherComp :type Primitive%20Component%20Object%20Reference) (OtherBodyIndex :type Integer) (bFromSweep :type Boolean) (SweepResult :type Hit%20Result%20Structure%20%28by%20ref%29))
  (bind _asflying_pawn (Utilities|Casting|CastToFlyingPawn OtherActor))
  (if (== (Variables|/Game/FlyingBP/Blueprints/FlyingPawn.FlyingPawn_C|Getcargobox _asflying_pawn) OtherComp)
    (Variables|/Game/FlyingBP/Blueprints/FlyingPawn.FlyingPawn_C|SetisInSafeCloud? _asflying_pawn true)))

(event OnComponentEndOverlap(Collider)
  (params (OverlappedComponent :type Primitive%20Component%20Object%20Reference) (OtherActor :type Actor%20Object%20Reference) (OtherComp :type Primitive%20Component%20Object%20Reference) (OtherBodyIndex :type Integer))
  (bind _asflying_pawn (Utilities|Casting|CastToFlyingPawn OtherActor))
  (if (== (Variables|/Game/FlyingBP/Blueprints/FlyingPawn.FlyingPawn_C|Getcargobox _asflying_pawn) OtherComp)
    (Variables|/Game/FlyingBP/Blueprints/FlyingPawn.FlyingPawn_C|SetisInSafeCloud? _asflying_pawn false)))

(event Custom|LightningOn
  (bind _returnvalue (Math|Random|RandomFloatinRange 5e+01 1e+02))
  (bind _lightning (Variables|Default|GetLightning))
  (bind _lightning_2 (Variables|Default|GetLightning))
  (bind _returnvalue_2 (Transformation|GetWorldLocation _lightning))
  (Components|Activation|Activate (Variables|Default|GetLightning) false)
  (Class|ParticleSystemComponent|SetBeamSourcePoint _lightning_2 0 (Transformation|GetWorldLocation _lightning_2))
  (Class|ParticleSystemComponent|SetBeamTargetPoint _lightning_2 0 (Math|Vector|MakeVector (+ (.x _returnvalue_2) _returnvalue) (+ (.y _returnvalue_2) _returnvalue) (- (.z _returnvalue_2) (Math|Random|RandomFloatinRange 1e+03 5e+03)))))

(event Custom|LIghtningOff
  (Components|Activation|Deactivate (Variables|Default|GetLightning)))

(event EventBeginPlay
  (for _array_element (Actor|GetComponentsbyTag "/Script/Engine.StaticMeshComponent" "Cloud")
    (Components|StaticMesh|SetStaticMesh _array_element (Utilities|Select :Index (Math|Random|RandomIntegerinRange 0 3) :Option%200 "/Game/NewClouds/SM_Cloud1.SM_Cloud1" :Option%201 "/Game/NewClouds/SM_Cloud2.SM_Cloud2" :Option%202 "/Game/NewClouds/SM_Cloud3.SM_Cloud3" :Option%203 "/Game/Meshes/SM_Cloud.SM_Cloud"))))

(event EventTick
  (params (DeltaSeconds :type Float%20%28single-precision%29))
  (if (Variables|Default|GetStormWLightning?)
    (Utilities|FlowControl|Delay (Math|Random|RandomFloatinRange 1.0 8.0))
    (CallFunction|Lightningon)
    (Utilities|FlowControl|Delay 0.2)
    (CallFunction|LIghtningOff)))

(fn ConstructionScript
  (if (Variables|Default|GetIsSafeCloud?)
    (for _array_element (Actor|GetComponentsbyTag "/Script/Engine.StaticMeshComponent" "Cloud")
      (Rendering|Material|SetMaterial _array_element 0 "/Game/Materials/cloud_blend_Inst_Safe.cloud_blend_Inst_Safe"))))