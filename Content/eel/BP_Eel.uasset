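; BP_Eel is an eel actor that swims in a curving path until it spots a FlyingPawn's cargo box.
; Tick applies forward movement and yaw while no player is spotted.
; When the Cargobox overlaps its Box, a timeline lerps the eel's root from its current location toward the pawn's mesh without sweeping.
; The spotted flag clears after a 15-second delay, resuming normal movement.
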(event OnComponentBeginOverlap(Box)
  (params (OverlappedComponent :type Primitive%20Component%20Object%20Reference) (OtherActor :type Actor%20Object%20Reference) (OtherComp :type Primitive%20Component%20Object%20Reference) (OtherBodyIndex :type Integer) (bFromSweep :type Boolean) (SweepResult :type Hit%20Result%20Structure%20%28by%20ref%29))
  (bind _asflying_pawn (Utilities|Casting|CastToFlyingPawn OtherActor))
  (Variables|Default|SetFlyingPawnTarget _asflying_pawn)
  (if (== (Variables|/Game/FlyingBP/Blueprints/FlyingPawn.FlyingPawn_C|Getcargobox _asflying_pawn) OtherComp)
    (Variables|Default|SetSpottedPlayer? true)
    (CallFunction|FlyingTowardsPlayer)
    (Utilities|FlowControl|Delay 15.0)
    (Variables|Default|SetSpottedPlayer? false)))

(event Custom|FlyingTowardsPlayer
  (bind _newtrack_0 (Timeline|Timeline_0 Play)
    (:Update
      (Transformation|SetWorldLocation (Variables|Default|GetDefaultSceneRoot) (Math|Vector|Lerp(Vector) (Transformation|GetWorldLocation (Variables|Default|GetDefaultSceneRoot)) (Transformation|GetWorldLocation (Variables|/Game/FlyingBP/Blueprints/FlyingPawn.FlyingPawn_C|GetSkeletalMesh (Variables|Default|GetFlyingPawnTarget))) _newtrack_0) false false))))

(event EventBeginPlay
  (Components|Animation|PlayAnimation (Variables|Default|GetSkeletalMesh) "/Game/eel/ANIM_Eel_slither.ANIM_Eel_slither" false))

(event Collision|EventActorBeginOverlap
  (params (OtherActor :type Actor%20Object%20Reference)))

(event EventTick
  (params (DeltaSeconds :type Float%20%28single-precision%29))
  (if (not (Variables|Default|GetSpottedPlayer?))
    (Transformation|AddActorLocalOffset (Math|Vector|MakeVector 0.0 (* DeltaSeconds (Variables|Default|GetForwardSpeed)) 0.0) false false)
    (Transformation|AddActorLocalRotation (Math|Rotator|MakeRotator 0.0 0.0 (* DeltaSeconds (Variables|Default|GetTurnSpeed))) false false)))

(fn ConstructionScript)