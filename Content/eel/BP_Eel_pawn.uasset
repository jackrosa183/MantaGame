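; BP_Eel_pawn is an eel pawn that loops a slither animation and pursues the player's flying pawn.
; A Box overlap with that pawn's Cargobox sets SpottedPlayer and issues an AI MoveTo toward it, then clears the flag after a 15-second delay.
; Tick holds forward-and-turn movement behind a constant branch condition that keeps it from running.
; The construction script yaws the skeletal mesh to -90 degrees.
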(event OnComponentBeginOverlap(Box)
  (params (OverlappedComponent :type Primitive%20Component%20Object%20Reference) (OtherActor :type Actor%20Object%20Reference) (OtherComp :type Primitive%20Component%20Object%20Reference) (OtherBodyIndex :type Integer) (bFromSweep :type Boolean) (SweepResult :type Hit%20Result%20Structure%20%28by%20ref%29))
  (bind _asflying_pawn (Utilities|Casting|CastToFlyingPawn OtherActor))
  (Variables|Default|SetFlyingPawnTaget _asflying_pawn)
  (if (== OtherComp (Variables|/Game/FlyingBP/Blueprints/FlyingPawn.FlyingPawn_C|Getcargobox _asflying_pawn))
    (Variables|Default|SetSpotted%20Player? true)
    (AI|AIMoveTo 0 "0, 0, 0" (Variables|Default|GetFlyingPawnTaget) 5.0 false
      (:then
        (Utilities|FlowControl|Delay 15.0)
        (Variables|Default|SetSpotted%20Player? false)))))

(event EventBeginPlay
  (Components|Animation|PlayAnimation (Variables|Default|GetSkeletalMesh) "/Game/eel/ANIM_Eel_slither.ANIM_Eel_slither" true))

(event EventTick
  (params (DeltaSeconds :type Float%20%28single-precision%29))
  (if (not true)
    (Transformation|AddActorLocalOffset (Math|Vector|MakeVector 0.0 (* DeltaSeconds (Variables|Default|GetForwardSpeed)) 0.0) false false)
    (Transformation|AddActorLocalRotation (Math|Rotator|MakeRotator 0.0 0.0 (* DeltaSeconds (Variables|Default|GetTurnSpeed))) false false)))

(fn ConstructionScript
  (Transformation|SetRelativeRotation (Variables|Default|GetSkeletalMesh) "0,-90.000000, 0" false false))