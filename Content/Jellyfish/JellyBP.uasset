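; Jellyfish actor Blueprint that plays a looping floating animation and drifts endlessly along its vertical axis.
; On BeginPlay, a MoveComponentTo eases the Jelly component up or down by a fixed offset from its current relative location.
; On completion, a FlipFlop sets the Repeat boolean that selects the next direction and re-enters the move, forming a latent loop without Tick.
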(event EventBeginPlay
  (bind _jelly (Variables|Default|GetJelly))
  (bind _relativelocation (Variables|/Script/Engine.SceneComponent|GetRelativeLocation _jelly))
  (Utilities|FlowControl|Sequence
    (:then_0
      (Components|Animation|PlayAnimation (Variables|Default|GetJelly) "/Game/Jellyfish/ANIM_Jellyfish_floating.ANIM_Jellyfish_floating" true))
    (:then_1
      (Components|MoveComponentTo _jelly (Math|Vector|SelectVector (+ _relativelocation "0, 0,200.000000") (- _relativelocation "0, 0,200.000000") (Variables|Default|Getrepeat)) "0, 0, 0" true true 8.0 false :!label _label)
      (Utilities|FlowControl|FlipFlop
        (:A
          (Variables|Default|Setrepeat true)
          (goto _label))
        (:B
          (Variables|Default|Setrepeat false)
          (goto _label))))))

(event Collision|EventActorBeginOverlap
  (params (OtherActor :type Actor%20Object%20Reference)))

(event EventTick
  (params (DeltaSeconds :type Float%20%28single-precision%29)))

(fn ConstructionScript)