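; Lionfish actor that swims continuously along a curving path, with no collision or interaction logic.
; On BeginPlay it loops the swimming animation at a randomized play rate so individual fish differ.
; Each Tick moves it along local Y by Speed and yaws it by TurnSpeed, both scaled by delta time and a random factor re-rolled every frame, without sweeping.
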(event EventBeginPlay
  (Components|Animation|PlayAnimation (Variables|Default|GetSkeletalMesh) "/Game/Lionfish/ANIM_Lionfish_swimming.ANIM_Lionfish_swimming" true)
  (Components|Timeline|SetPlayRate (Variables|Default|GetSkeletalMesh) (Math|Random|RandomFloatinRange 0.8 1.2)))

(event Collision|EventActorBeginOverlap
  (params (OtherActor :type Actor%20Object%20Reference)))

(event EventTick
  (params (DeltaSeconds :type Float%20%28single-precision%29))
  (bind _returnvalue (Math|Random|RandomFloatinRange 0.8 1.2))
  (Transformation|AddActorLocalOffset (Math|Vector|MakeVector 0.0 (* (* DeltaSeconds (Variables|Default|Getspeed)) _returnvalue) 0.0) false false)
  (Transformation|AddActorLocalRotation (Math|Rotator|MakeRotator 0.0 0.0 (* (* DeltaSeconds (Variables|Default|GetTurnSpeed)) _returnvalue)) false false))

(fn ConstructionScript)